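; Boids flock actor that renders boids as mesh instances on ISMComp; no flocking logic is in this graph.
; Construction copies the initial count and spread radius and assigns the mesh.
; A looping timer randomizes per-instance custom data for colors, while Tick draws the spread sphere and optional per-boid proximity spheres.
; AddMoreInstances forwards to AddInstances; RemoveExtraInstances is empty, with older Blueprint add/remove logic left disconnected as unsupported.
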(event EventBeginPlay
  (|CallParentFunction)
  ;[1 0.5742 0.8013] Update Custom Data is used to set random colors
  (Utilities|Time|SetTimerbyFunctionName 0 "UpdateCustomData" 0.3 true))

(event EventTick
  (params (DeltaSeconds :type Float%20%28single-precision%29))
  (bind _spreadradius (Variables|Default|GetSpreadRadius))
  (|CallParentFunction DeltaSeconds)
  ;[1 1 1] Debug helpers to visualize Spread Radius
  (Rendering|Debug|DrawDebugSphere (Transformation|GetActorLocation) _spreadradius 8 "(R=0.532986,G=0.714460,B=1.000000,A=1.000000)" 0.0)
  (if (Variables|Default|GetbToggleProximityDebug)
    (Development|PrintString (Utilities|String|Append "Spread Radius: " (Utilities|String|ToString(Float) _spreadradius)) true false "(R=0.000000,G=1.000000,B=0.613023,A=1.000000)" 0.0)
    ;[0.3928 0.7282 1] Draw debug helpers to visualize each boid's Proximity Sensor's radius
    (for (_ _array_index) (Variables|Default|GetInstanceIndices)
      (Rendering|Debug|DrawDebugSphere (.location (.OutInstanceTransform (Components|InstancedStaticMesh|GetInstanceTransform (Variables|Default|GetISMComp) _array_index true))) (Variables|Default|GetProximityRadius) 4 "(R=0.509107,G=0.000000,B=0.904514,A=1.000000)" 0.0))))

(fn ConstructionScript
  ;[1 1 1] Warning! It is important not to set directly NumInstances of Spaw, program will crash. Please use AddMore / RemoveExtra Functions
  (Variables|Default|SetNumInstances (Variables|Default|GetInitNumInstances))
  (Variables|Default|SetSpreadRadius (Variables|Default|GetInitSpreadRadius))
  ;[0.811 1 0.6354] Initial mesh is set from UI
  (Components|StaticMesh|SetStaticMesh (Variables|Default|GetISMComp) (Variables|Default|GetStaticMeshToSpawn)))

(fn AddMoreInstances
  (params (NumToAdd :type Integer))
  (Class|BFlock|AddInstances NumToAdd))

(fn RemoveExtraInstances
  (params (InstancesToRemove :type Integer)))

(fn UpdateCustomData
  (for (_ _array_index) (Variables|Default|GetInstanceIndices)
    (Components|InstancedStaticMesh|SetCustomDataValue (Variables|Default|GetISMComp) _array_index 0 (Math|Random|RandomFloatinRange 0.0 0.3) false)
    (Components|InstancedStaticMesh|SetCustomDataValue (Variables|Default|GetISMComp) _array_index 1 (Math|Random|RandomFloatinRange 0.0 0.05) false)
    (Components|InstancedStaticMesh|SetCustomDataValue (Variables|Default|GetISMComp) _array_index 2 (Math|Random|RandomFloatinRange 0.05 0.2) false)))